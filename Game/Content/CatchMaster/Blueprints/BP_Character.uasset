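; Player character for CatchMaster that slides a cube sideways along the world Y axis and wraps it between screen sides.
; The Move Right axis value is stored, then scaled by a fixed per-frame step on Tick and added to the cube's current Y.
; Crossing either boundary teleports the cube just inside the opposite side, with no sweep and no delta-time scaling.
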(event EventTick
  (params (DeltaSeconds :type Float%20%28single-precision%29))
  (bind _cube (Variables|Default|GetCube))
  (bind _cube_2 (Variables|Default|GetCube))
  (bind _returnvalue (Transformation|GetWorldLocation _cube_2))
  (bind _returnvalue_2 (Transformation|GetWorldLocation _cube))
  ;[1 1 1] Movement and Teleportation of Player
  (bind _output_get (Variables|Default|SetMovementOffset (+ (* (Variables|Default|GetMovementOffset) 25.0) (.y _returnvalue_2))))
  (if (and (< _output_get 6.5e+02) (> _output_get -6.5e+02))
    (Transformation|SetWorldLocation _cube (Math|Vector|MakeVector (.x _returnvalue_2) _output_get (.z _returnvalue_2)) false false)
    (elif (>= _output_get 6.5e+02)
      (Transformation|SetWorldLocation _cube_2 (Math|Vector|MakeVector (.x _returnvalue) -599.0 (.z _returnvalue)) false false)
      (elif (<= _output_get -6.5e+02)
        (Transformation|SetWorldLocation _cube_2 (Math|Vector|MakeVector (.x _returnvalue) 599.0 (.z _returnvalue)) false false)))))

(event Input|AxisEvents|InputAxisMoveRight
  (params (AxisValue :type Float%20%28single-precision%29))
  ;[1 1 1] Movement and Teleportation of Player
  (Variables|Default|SetMovementOffset AxisValue))

(fn ConstructionScript)