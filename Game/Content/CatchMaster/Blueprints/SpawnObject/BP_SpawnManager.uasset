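; BP_SpawnManager spawns falling-object candidates for CatchMaster at a random horizontal position in a high band whenever CrystalSpawn is called.
; ChooseRarity makes a weighted random roll over the RarityMap in BP_ObjectInst, the game instance, by summing weights then subtracting until one covers the roll.
; One rarity value spawns a BP_Stalagmite, while every other spawns an item actor carrying that rarity in its item details.
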(event Custom|CrystalSpawn
  (bind _returnvalue (Math|Random|RandomFloatinRange -5.5e+02 5.5e+02))
  (bind _returnvalue_2 (Math|Random|RandomFloatinRange 8e+02 8.5e+02))
  (bind _returnvalue_3 (Math|Vector|MakeVector 0.0 _returnvalue _returnvalue_2))
  (bind _rarity (CallFunction|ChooseRarity))
  (if (Utilities|Enum|NotEqual(Enum) _rarity "NewEnumerator4")
    (Game|SpawnActorfromClass "/Game/CatchMaster/Blueprints/SpawnObject/BP_Crystal_Item.BP_Crystal_Item_C" (Math|Transform|MakeTransform _returnvalue_3 "0, 0, 0" "1.000000,1.000000,1.000000") "AdjustIfPossibleButAlwaysSpawn" "MultiplyWithRoot" 0 (Utilities|Struct|MakeSTRUCT_Item _rarity) 0)
    (else
      (Game|SpawnActorfromClass "/Game/CatchMaster/Blueprints/SpawnObject/BP_Stalagmite.BP_Stalagmite_C" (Math|Transform|MakeTransform _returnvalue_3 "0, 0, 0" "1.000000,1.000000,1.000000") "Undefined" "MultiplyWithRoot" 0 0))))

(fn ConstructionScript)

(fn ChooseRarity
  (bind _asbp_object_inst (Utilities|Casting|CastToBP_ObjectInst (Game|GetGameInstance)))
  (bind _keys (Utilities|Map|Keys (Variables|/Game/CatchMaster/Blueprints/SpawnObject/BP_ObjectInst.BP_ObjectInst_C|GetRarityMap _asbp_object_inst)))
  (for _array_element _keys
    (LocalVariables|SetSumOfRarity (+ (.Value (Utilities|Map|Find (Variables|/Game/CatchMaster/Blueprints/SpawnObject/BP_ObjectInst.BP_ObjectInst_C|GetRarityMap _asbp_object_inst) _array_element)) (LocalVariables|GetSumOfRarity))))
  (LocalVariables|SetCrystalRool (Math|Random|RandomFloatinRange 0.0 (LocalVariables|GetSumOfRarity)))
  (bind _keys_2 (Utilities|Map|Keys (Variables|/Game/CatchMaster/Blueprints/SpawnObject/BP_ObjectInst.BP_ObjectInst_C|GetRarityMap _asbp_object_inst)))
  (bind _array_element_2 (Utilities|Array|ForEachLoopwithBreak _keys_2 :!label _label)
    (:LoopBody
      (if (>= (.Value (Utilities|Map|Find (Variables|/Game/CatchMaster/Blueprints/SpawnObject/BP_ObjectInst.BP_ObjectInst_C|GetRarityMap _asbp_object_inst) _array_element_2)) (LocalVariables|GetCrystalRool))
        (LocalVariables|SetRarityOut _array_element_2)
        (goto _label Break)
        (else
          (LocalVariables|SetCrystalRool (- (LocalVariables|GetCrystalRool) (.Value (Utilities|Map|Find (Variables|/Game/CatchMaster/Blueprints/SpawnObject/BP_ObjectInst.BP_ObjectInst_C|GetRarityMap _asbp_object_inst) _array_element_2)))))))
    (:Completed
      (return (LocalVariables|GetRarityOut)))))