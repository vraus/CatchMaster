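; Player character for a catch game, sliding a cube sideways to collect falling crystals.
; Tick applies the Move Right axis to the cube's Y position, wrapping it to the opposite side at the play-area edges.
; Overlaps identify crystals by mesh component name and pick points from material, passing them to the PlayerHUD widget.
; Each catch also decrements GM_Gamemode's live-object count, triggers its round-end check and destroys the crystal.
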(event OnComponentBeginOverlap(PlayerCollision)
  (params (OverlappedComponent :type Primitive%20Component%20Object%20Reference) (OtherActor :type Actor%20Object%20Reference) (OtherComp :type Primitive%20Component%20Object%20Reference) (OtherBodyIndex :type Integer) (bFromSweep :type Boolean) (SweepResult :type Hit%20Result%20Structure%20%28by%20ref%29))
  (bind _returnvalue (Actor|GetComponentbyClass OtherActor "/Script/Engine.StaticMeshComponent"))
  ;[1 1 1] Collision Betwen Player and Falling Object
  (Variables|Default|SetCrystalB _returnvalue)
  (if (Utilities|String|Contains (Utilities|GetObjectName _returnvalue) "Crystal_Blue")
    ;;[1 1 1] Score
    (bind _foundwidgets (Widget|GetAllWidgetsOfClass "/Game/CatchMaster/Blueprints/HUD/PlayerHUD.PlayerHUD_C" true))
    (Default|IncreasePoint (Utilities|Array|Get(acopy) _foundwidgets) (Math|Integer|SelectInt 10 (Math|Integer|SelectInt 20 (Math|Integer|SelectInt 30 40 (== (Rendering|Material|GetMaterial (Variables|Default|GetCrystalB) 0) "/Game/CatchMaster/Material/Green.Green")) (== (Rendering|Material|GetMaterial (Variables|Default|GetCrystalB) 0) "/Game/CatchMaster/Material/Red.Red")) (== (Rendering|Material|GetMaterial (Variables|Default|GetCrystalB) 0) "/Game/CatchMaster/Material/Blue1.Blue1")))
    ;;[1 1 1] Delete Falling Objects
    (bind _asgm_gamemode (Utilities|Casting|CastToGM_Gamemode (Game|GetGameMode)))
    (Math|Integer|DecrementInt (Variables|/Game/CatchMaster/Blueprints/GM_Gamemode.GM_Gamemode_C|GetObject_Alive _asgm_gamemode)
      (:%20%20
        (Default|ChekifRoundEnd _asgm_gamemode)
        (Actor|DestroyActor (Components|GetOwner (Variables|Default|GetCrystalB)))))))

(event EventTick
  (params (DeltaSeconds :type Float%20%28single-precision%29))
  (bind _cube (Variables|Default|GetCube))
  (bind _cube_2 (Variables|Default|GetCube))
  (bind _returnvalue (Transformation|GetWorldLocation _cube))
  (bind _returnvalue_2 (Transformation|GetWorldLocation _cube_2))
  ;[1 1 1] Movement and Teleportation of Player
  (bind _output_get (Variables|Default|SetMovementOffset (+ (* (Variables|Default|GetMovementOffset) 15.0) (.y _returnvalue))))
  (if (and (< _output_get 6.5e+02) (> _output_get -6.5e+02))
    (Transformation|SetWorldLocation _cube (Math|Vector|MakeVector (.x _returnvalue) _output_get (.z _returnvalue)) false false)
    (elif (>= _output_get 6.5e+02)
      (Transformation|SetWorldLocation _cube_2 (Math|Vector|MakeVector (.x _returnvalue_2) -599.0 (.z _returnvalue_2)) false false)
      (elif (<= _output_get -6.5e+02)
        (Transformation|SetWorldLocation _cube_2 (Math|Vector|MakeVector (.x _returnvalue_2) 599.0 (.z _returnvalue_2)) false false)))))

(event Input|AxisEvents|InputAxisMoveRight
  (params (AxisValue :type Float%20%28single-precision%29))
  ;[1 1 1] Movement and Teleportation of Player
  (Variables|Default|SetMovementOffset AxisValue))

(fn ConstructionScript)