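; LoosingZone is a trigger volume that removes falling blue crystals that reach it.
; On Box overlap, it identifies crystals by searching the other actor's static mesh component name for "Crystal_Blue", rather than casting to a class.
; For a match, it decrements ObjectAlive on GM_Gamemode, calls ChekIfRoundEnd, then destroys the crystal's owning actor.
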(event OnComponentBeginOverlap(Box)
  (params (OverlappedComponent :type Primitive%20Component%20Object%20Reference) (OtherActor :type Actor%20Object%20Reference) (OtherComp :type Primitive%20Component%20Object%20Reference) (OtherBodyIndex :type Integer) (bFromSweep :type Boolean) (SweepResult :type Hit%20Result%20Structure%20%28by%20ref%29))
  (bind _returnvalue (Actor|GetComponentbyClass OtherActor "/Script/Engine.StaticMeshComponent"))
  (Variables|Default|SetCrystal _returnvalue)
  (if (Utilities|String|Contains (Utilities|GetObjectName _returnvalue) "Crystal_Blue")
    ;[1 1 1] Delete Falling Objects
    (bind _asgm_gamemode (Utilities|Casting|CastToGM_Gamemode (Game|GetGameMode)))
    (Math|Integer|DecrementInt (Variables|/Game/CatchMaster/Blueprints/GM_Gamemode.GM_Gamemode_C|GetObject_Alive _asgm_gamemode)
      (:%20%20
        (Default|ChekifRoundEnd _asgm_gamemode)
        (Actor|DestroyActor (Components|GetOwner (Variables|Default|GetCrystal)))))))

(fn ConstructionScript)