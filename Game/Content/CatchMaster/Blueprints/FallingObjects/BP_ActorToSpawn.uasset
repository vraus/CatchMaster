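; BP_ActorToSpawn is a falling object in CatchMaster that awards points when the player catches it.
; Its sphere overlap tells hits apart by searching the other actor's box component name for "Box" or "PlayerCollision".
; A player hit first increases points on the PlayerHUD widget.
; Both hit types then decrement GM_Gamemode's live object count, trigger its round-end check and destroy the actor.
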(event OnComponentBeginOverlap(Sphere)
  (params (OverlappedComponent :type Primitive%20Component%20Object%20Reference) (OtherActor :type Actor%20Object%20Reference) (OtherComp :type Primitive%20Component%20Object%20Reference) (OtherBodyIndex :type Integer) (bFromSweep :type Boolean) (SweepResult :type Hit%20Result%20Structure%20%28by%20ref%29))
  ;[1 1 1] Check the Component in Collision
  (if (Utilities|String|Contains (Utilities|GetObjectName (Actor|GetComponentbyClass OtherActor "/Script/Engine.BoxComponent")) "Box")
    ;[1 1 1] Delete Falling Objects
    (bind _asgm_gamemode (Utilities|Casting|CastToGM_Gamemode (Game|GetGameMode) :!label _label))
    (Math|Integer|DecrementInt (Variables|/Game/CatchMaster/Blueprints/GM_Gamemode.GM_Gamemode_C|GetObject_Alive _asgm_gamemode)
      (:%20%20
        (Default|ChekifRoundEnd _asgm_gamemode)
        (Actor|DestroyActor)))
    (elif (Utilities|String|Contains (Utilities|GetObjectName (Actor|GetComponentbyClass OtherActor "/Script/Engine.BoxComponent")) "PlayerCollision")
      ;[1 1 1] Score
      (bind _foundwidgets (Widget|GetAllWidgetsOfClass "/Game/CatchMaster/Blueprints/HUD/PlayerHUD.PlayerHUD_C" true))
      (Default|IncreasePoint (Utilities|Array|Get(acopy) _foundwidgets) (Math|Integer|SelectInt 10 10 false))
      (goto _label))))

(fn ConstructionScript)