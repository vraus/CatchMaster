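; Spawn manager for falling objects in CatchMaster that creates a BP_BlueCrystal whenever its Spawn event is called.
; Each crystal appears at a random Y and height on the X=0 plane.
; Chained random checks set its material to none (mesh default), Red, Green or Black, with weights that appear intended to favor the default.
; Each check calls RandomInteger separately rather than sharing one roll, so the actual odds differ from a seven-way split.
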(event Custom|Spawn
  (bind _returnvalue (Math|Random|RandomInteger 7))
  (bind _returnvalue_2 (Game|SpawnActorfromClass "/Game/CatchMaster/Blueprints/FallingObjects/BP_BlueCrystal.BP_BlueCrystal_C" (Math|Transform|MakeTransform (Math|Vector|MakeVector 0.0 (Math|Random|RandomFloatinRange -5.5e+02 5.5e+02) (Math|Random|RandomFloatinRange 8e+02 8.5e+02)) "0, 0, 0" "1.000000,1.000000,1.000000") "Undefined" "MultiplyWithRoot" 0 0))
  (if (or (or (== _returnvalue 0) (== _returnvalue 1)) (== _returnvalue 2))
    (Rendering|Material|SetMaterial (Variables|/Game/CatchMaster/Blueprints/FallingObjects/BP_BlueCrystal.BP_BlueCrystal_C|GetCrystal_Blue _returnvalue_2) 0 0)
    (elif (or (== _returnvalue 3) (== _returnvalue 4))
      (Rendering|Material|SetMaterial (Variables|/Game/CatchMaster/Blueprints/FallingObjects/BP_BlueCrystal.BP_BlueCrystal_C|GetCrystal_Blue _returnvalue_2) 0 "/Game/CatchMaster/Material/Red.Red")
      (elif (== _returnvalue 5)
        (Rendering|Material|SetMaterial (Variables|/Game/CatchMaster/Blueprints/FallingObjects/BP_BlueCrystal.BP_BlueCrystal_C|GetCrystal_Blue _returnvalue_2) 0 "/Game/CatchMaster/Material/Green.Green")
        (else
          (Rendering|Material|SetMaterial (Variables|/Game/CatchMaster/Blueprints/FallingObjects/BP_BlueCrystal.BP_BlueCrystal_C|GetCrystal_Blue _returnvalue_2) 0 "/Game/CatchMaster/Material/Black.Black"))))))

(fn ConstructionScript)